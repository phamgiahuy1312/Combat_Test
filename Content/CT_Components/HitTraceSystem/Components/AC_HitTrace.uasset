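; Actor component that runs named hit-detection traces between two mesh sockets, ticking only while tasks are active.
; BeginTrace functions register tasks by channel, object type or profile; EndTrace clears them.
; Each tick sweeps an oriented box between the midpoints of previous and current socket positions, sized by start-socket travel to cover inter-frame gaps.
; OnHitActor fires once per actor per task, deduplicated by display name.
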(event `self.ReceiveTick`
  (params (DeltaSeconds :type "Float (single-precision)"))
  (bind _keys (`BlueprintMapLibrary.Map_Keys` (`self.TraceDataMap`)))
  (for _array_element _keys
    (`self.TryTrace` _array_element)))

(fn `BeginTraceByChannel`
  (params (TaskName :type Name) (Mesh :type "SceneComponent Object Reference") (BeginSocket :type Name) (EndSocket :type Name) (IgnoreActors :type "Array of Actor Object Reference") (Radius :type "Float (double-precision)" :default 1.0) (TraceChannel :type "ETraceTypeQuery Enum" :default "TraceTypeQuery1") (TraceComplex :type Boolean) (DrawDebugType :type "EDrawDebugTrace Enum" :default "None") (IgnoreSelf :type Boolean :default true) (Instigator :type "Actor Object Reference"))
  (`BlueprintMapLibrary.Map_Add` (`self.TraceDataMap`) (`local.TaskName`) (make `/Game/CT_Components/HitTraceSystem/Structs/CT_Struct_TraceData` :`Mesh` (`local.Mesh`) :`BeginSocket` (`local.BeginSocket`) :`EndSocket` (`local.EndSocket`) :`TraceChannel` (`local.TraceChannel`) :`ObjectTypes` (`|MakeArray` "ObjectTypeQuery1" :!type "EObjectTypeQuery Enum") :`TraceComplex` (`local.TraceComplex`) :`IgnoreActors` (`local.IgnoreActors`) :`Radius` (`local.Radius`) :`DrawDebugType` (`local.DrawDebugType`) :`IgnoreSelf` (`local.IgnoreSelf`) :`Instigator` (`local.Instigator`)))
  (`self.SetComponentTickEnabled` true))

(fn `BeginTraceByObjects`
  (params (TaskName :type Name) (Mesh :type "SceneComponent Object Reference") (BeginSocket :type Name) (EndSocket :type Name) (IgnoreActors :type "Array of Actor Object Reference") (Radius :type "Float (double-precision)" :default 1.0) (ObjectTypes :type "Array of EObjectTypeQuery Enum") (TraceComplex :type Boolean) (DrawDebugType :type "EDrawDebugTrace Enum" :default "None") (IgnoreSelf :type Boolean :default true) (Instigator :type "Actor Object Reference"))
  (`BlueprintMapLibrary.Map_Add` (`self.TraceDataMap`) (`local.TaskName`) (make `/Game/CT_Components/HitTraceSystem/Structs/CT_Struct_TraceData` :`Mesh` (`local.Mesh`) :`TraceType` "NewEnumerator1" :`BeginSocket` (`local.BeginSocket`) :`EndSocket` (`local.EndSocket`) :`ObjectTypes` (`local.ObjectTypes`) :`TraceComplex` (`local.TraceComplex`) :`IgnoreActors` (`local.IgnoreActors`) :`Radius` (`local.Radius`) :`DrawDebugType` (`local.DrawDebugType`) :`IgnoreSelf` (`local.IgnoreSelf`) :`Instigator` (`local.Instigator`)))
  (`self.SetComponentTickEnabled` true))

(fn `BeginTraceByProfile`
  (params (TaskName :type Name) (Mesh :type "SceneComponent Object Reference") (BeginSocket :type Name) (EndSocket :type Name) (IgnoreActors :type "Array of Actor Object Reference") (Radius :type "Float (double-precision)" :default 1.0) (ProfileName :type Name) (TraceComplex :type Boolean) (DrawDebugType :type "EDrawDebugTrace Enum" :default "None") (IgnoreSelf :type Boolean :default true) (Instigator :type "Actor Object Reference"))
  (`BlueprintMapLibrary.Map_Add` (`self.TraceDataMap`) (`local.TaskName`) (make `/Game/CT_Components/HitTraceSystem/Structs/CT_Struct_TraceData` :`Mesh` (`local.Mesh`) :`TraceType` "NewEnumerator2" :`BeginSocket` (`local.BeginSocket`) :`EndSocket` (`local.EndSocket`) :`ObjectTypes` (`|MakeArray` "ObjectTypeQuery1" :!type "EObjectTypeQuery Enum") :`ProfileName` (`local.ProfileName`) :`TraceComplex` (`local.TraceComplex`) :`IgnoreActors` (`local.IgnoreActors`) :`Radius` (`local.Radius`) :`DrawDebugType` (`local.DrawDebugType`) :`IgnoreSelf` (`local.IgnoreSelf`) :`Instigator` (`local.Instigator`)))
  (`self.SetComponentTickEnabled` true))

(fn `CheckActorIsFirstTrace`
  (params (Actor :type "Actor Object Reference") (TaskName :type Name))
  (returns (Result :type Boolean))
  (locals (Local_ActorName :type String) (Local_Map :type "Map of String to Boolean") (Local_TraceData :type "/Game/CT_Components/HitTraceSystem/Structs/CT_Struct_TraceData Structure"))
  (bind _value (`BlueprintMapLibrary.Map_Find` (`self.TraceDataMap`) (`local.TaskName`)))
  (set `local.Local_ActorName` (`KismetSystemLibrary.GetDisplayName` Actor))
  (set `local.Local_TraceData` _value)
  (set `local.Local_Map` (`.TracedMap_40_269D44974E871EBD3D16B59307A58238` (break `/Game/CT_Components/HitTraceSystem/Structs/CT_Struct_TraceData` _value)))
  (`/Engine/EditorBlueprintResources/StandardMacros.IsValid` (`local.Actor`)
    (:`Is Valid`
      (if (`BlueprintMapLibrary.Map_Contains` (`local.Local_Map`) (`local.Local_ActorName`))
        (return false)
        (else
          (`BlueprintMapLibrary.Map_Add` (`local.Local_Map`) (`local.Local_ActorName`) true)
          (setmembers `/Game/CT_Components/HitTraceSystem/Structs/CT_Struct_TraceData` :`StructRef` (`local.Local_TraceData`) :`TracedMap` (`local.Local_Map`))
          (`BlueprintMapLibrary.Map_Add` (`self.TraceDataMap`) (`local.TaskName`) (`local.Local_TraceData`))
          (return true))))
    (:`Is Not Valid`
      (return false))))

(fn `EndTrace`
  (params (TaskName :type Name))
  (`BlueprintMapLibrary.Map_Remove` (`self.TraceDataMap`) (`local.TaskName`))
  (`BlueprintMapLibrary.Map_Remove` (`self.LastStartLocationMap`) (`local.TaskName`))
  (`BlueprintMapLibrary.Map_Remove` (`self.LastEndLocationMap`) (`local.TaskName`))
  (if (`BlueprintMapLibrary.Map_IsEmpty` (`self.TraceDataMap`))
    (`self.SetComponentTickEnabled` false)))

(fn `MakeBoxTrace`
  (params (TaskName :type Name) (Start :type "Vector Structure") (End :type "Vector Structure") (HalfSize :type "Vector Structure") (Orientation :type "Rotator Structure"))
  (locals (TempHitResults :type "Array of HitResult Structure") (Local_OutActors :type "Array of Actor Object Reference") (Local_OutHits :type "Array of HitResult Structure") (Local_TraceData :type "/Game/CT_Components/HitTraceSystem/Structs/CT_Struct_TraceData Structure"))
  (bind ((`Mesh_22_D04901CA45F707BCE85B8F87B470F223` _mesh) (`Instigator_44_D522873740AC225F4322CC9F413655D1` _instigator)) (break `/Game/CT_Components/HitTraceSystem/Structs/CT_Struct_TraceData` (`local.Local_TraceData`)))
  (bind ((`ProfileName_32_61B2451A4AE57DF4E5213F80EA782CA0` _profilename) (`TraceComplex_16_D42B6FA64D8D397B9B498B835BC155C4` _tracecomplex) (`IgnoreActors_26_250F121948F1310D38005DBDC3B620FC` _ignoreactors) (`DrawDebugType_28_CDD89BB24AB468F4CF3A9ABA23955BE8` _drawdebugtype) (`IgnoreSelf_17_D57F68D94834F40CE3A122AD98AD8AB1` _ignoreself)) (break `/Game/CT_Components/HitTraceSystem/Structs/CT_Struct_TraceData` (`local.Local_TraceData`)))
  (bind ((`TraceChannel_29_A4FBBE864552FD6497A9D794D2D128ED` _tracechannel) (`TraceComplex_16_D42B6FA64D8D397B9B498B835BC155C4` _tracecomplex_2) (`IgnoreActors_26_250F121948F1310D38005DBDC3B620FC` _ignoreactors_2) (`DrawDebugType_28_CDD89BB24AB468F4CF3A9ABA23955BE8` _drawdebugtype_2) (`IgnoreSelf_17_D57F68D94834F40CE3A122AD98AD8AB1` _ignoreself_2)) (break `/Game/CT_Components/HitTraceSystem/Structs/CT_Struct_TraceData` (`local.Local_TraceData`)))
  (bind ((`ObjectTypes_31_DBA7033E4A1E8DD5A9D14EBCD3BA793B` _objecttypes) (`TraceComplex_16_D42B6FA64D8D397B9B498B835BC155C4` _tracecomplex_3) (`IgnoreActors_26_250F121948F1310D38005DBDC3B620FC` _ignoreactors_3) (`DrawDebugType_28_CDD89BB24AB468F4CF3A9ABA23955BE8` _drawdebugtype_3) (`IgnoreSelf_17_D57F68D94834F40CE3A122AD98AD8AB1` _ignoreself_3)) (break `/Game/CT_Components/HitTraceSystem/Structs/CT_Struct_TraceData` (`local.Local_TraceData`)))
  (set `local.Local_TraceData` (`BlueprintMapLibrary.Map_Find` (`self.TraceDataMap`) (`local.TaskName`)))
  (switch `/Game/CT_Components/HitTraceSystem/Enums/CT_Enum_TraceType` (`.TraceType_35_687E3B994EC27A1D6B06219A67306CC4` (break `/Game/CT_Components/HitTraceSystem/Structs/CT_Struct_TraceData` (`local.Local_TraceData`)))
    (:`NewEnumerator0`
      (bind _outhits (`KismetSystemLibrary.BoxTraceMulti` (`local.Start`) (`local.End`) (`local.HalfSize`) (`local.Orientation`) _tracechannel _tracecomplex_2 _ignoreactors_2 _drawdebugtype_2 _ignoreself_2))
      (set `local.Local_OutHits` _outhits))
    (:`NewEnumerator1`
      (bind _outhits_2 (`KismetSystemLibrary.BoxTraceMultiForObjects` (`local.Start`) (`local.End`) (`local.HalfSize`) (`local.Orientation`) _objecttypes _tracecomplex_3 _ignoreactors_3 _drawdebugtype_3 _ignoreself_3))
      (set `local.Local_OutHits` _outhits_2))
    (:`NewEnumerator2`
      (bind _outhits_3 (`KismetSystemLibrary.BoxTraceMultiByProfile` (`local.Start`) (`local.End`) (`local.HalfSize`) (`local.Orientation`) _profilename _tracecomplex _ignoreactors _drawdebugtype _ignoreself))
      (set `local.Local_OutHits` _outhits_3)))
  (for _array_element (`local.Local_OutHits`)
    (bind (_bblockinghit _binitialoverlap _time _distance _location _impactpoint _normal _impactnormal _physmat _hitactor) (`GameplayStatics.BreakHitResult` _array_element))
    (`/Engine/EditorBlueprintResources/StandardMacros.IsValid` _hitactor
      (:`Is Valid`
        (if (`self.CheckActorIsFirstTrace` _hitactor (`local.TaskName`))
          (`self.Event_OnHitActor` (`local.TaskName`) _mesh _instigator _hitactor _array_element))))))

(fn `TryTrace`
  (params (TaskName :type Name))
  (locals (Local_StartLocation :type "Vector Structure" :default (0.0 0.0 0.0)) (Local_EndLocation :type "Vector Structure" :default (0.0 0.0 0.0)) (Local_TraceData :type "/Game/CT_Components/HitTraceSystem/Structs/CT_Struct_TraceData Structure") (Local_LastStartLocation :type "Vector Structure") (Local_LastEndLocation :type "Vector Structure"))
  (bind ((`Radius_27_067E32F44F39EB9A1E3CE9B6938CE2F0` _radius)) (break `/Game/CT_Components/HitTraceSystem/Structs/CT_Struct_TraceData` (`local.Local_TraceData`)))
  (bind ((`Mesh_22_D04901CA45F707BCE85B8F87B470F223` _mesh) (`BeginSocket_23_0031ED714EA9891C09FFB38118BA8137` _beginsocket) (`EndSocket_24_B171BCA240B33906511A7DB02D4BBC60` _endsocket)) (break `/Game/CT_Components/HitTraceSystem/Structs/CT_Struct_TraceData` (`local.Local_TraceData`)))
  (bind (_value _returnvalue) (`BlueprintMapLibrary.Map_Find` (`self.TraceDataMap`) (`local.TaskName`)))
  (set `local.Local_TraceData` _value)
  (if _returnvalue
    (set `local.Local_StartLocation` (`SceneComponent.GetSocketLocation` _mesh _beginsocket))
    (set `local.Local_EndLocation` (`SceneComponent.GetSocketLocation` _mesh _endsocket))
    (set `local.Local_LastStartLocation` (`BlueprintMapLibrary.Map_Find` (`self.LastStartLocationMap`) (`local.TaskName`)))
    (set `local.Local_LastEndLocation` (`BlueprintMapLibrary.Map_Find` (`self.LastEndLocationMap`) (`local.TaskName`)))
    (`|ExecutionSequence`
      (:`then_0`
        (if (`KismetMathLibrary.EqualExactly_VectorVector` (+ (`local.Local_LastStartLocation`) (`local.Local_LastEndLocation`)))
          (`BlueprintMapLibrary.Map_Add` (`self.LastStartLocationMap`) (`local.TaskName`) (`local.Local_StartLocation`))
          (`BlueprintMapLibrary.Map_Add` (`self.LastEndLocationMap`) (`local.TaskName`) (`local.Local_EndLocation`))
          (return)))
      (:`then_1`
        (`self.MakeBoxTrace` (`local.TaskName`) (/ (+ (`local.Local_StartLocation`) (`local.Local_LastStartLocation`)) 2.0) (/ (+ (`local.Local_EndLocation`) (`local.Local_LastEndLocation`)) 2.0) (`KismetMathLibrary.MakeVector` (/ (`KismetMathLibrary.Vector_Distance` (`local.Local_LastStartLocation`) (`local.Local_StartLocation`)) 2.0) _radius _radius) (`KismetMathLibrary.FindLookAtRotation` (`local.Local_LastStartLocation`) (`local.Local_StartLocation`))))
      (:`then_2`
        (`BlueprintMapLibrary.Map_Add` (`self.LastStartLocationMap`) (`local.TaskName`) (`local.Local_StartLocation`))
        (`BlueprintMapLibrary.Map_Add` (`self.LastEndLocationMap`) (`local.TaskName`) (`local.Local_EndLocation`))))))