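; Anim notify state that marks a combo attack window in a montage or animation and applies melee hits to BP_AI enemies.
; Begin opens the owner's AC_Combo window and hitbox, then binds to AC_HitTrace to collect unique AI hit.
; End closes both, calls PlayNextCombo, then applies deferred damage, directional launch from the character capsule and blood VFX to collected AI, with hit or miss sound.
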(fn `Event_OnHitActor`
  (params (TaskName :type Name) (Mesh :type "SceneComponent Object Reference") (Instigator :type "Actor Object Reference") (Actor :type "Actor Object Reference") (HitResult :type "HitResult Structure"))
  (bind _asbp_ai (cast `/Game/ComboGame/Character/BP_AI` Actor))
  (`KismetArrayLibrary.Array_AddUnique` (`self.As BP AI`) _asbp_ai))

(fn `Hit ACtion`
  (params (Lauch :type "Vector Structure") (Weapon :type Boolean) (Actor :type "Actor Object Reference"))
  (if (`KismetArrayLibrary.Array_IsNotEmpty` (`self.As BP AI`))
    (for _array_element (`self.As BP AI`)
      (`/Engine/EditorBlueprintResources/StandardMacros.IsValid` _array_element
        (:`Is Valid`
          (`/Game/ComboGame/Character/BP_AI.Hit Action` _array_element (`self.Dame`) (`local.Lauch`) (`local.Weapon`))
          (`/Game/ComboGame/Character/BP_AI.Hit VFX Blood` _array_element))))
    (`/Game/ComboGame/Character/BP_AI.Play Sound Hit` _array_element (`local.Weapon`))
    (else
      (`/Game/ComboGame/Blueprint/AC_Combo.Play Sound Not Hit` (`Actor.GetComponentByClass` Actor "/Game/ComboGame/Blueprint/AC_Combo.AC_Combo_C") (`local.Weapon`)))))

(fn `Lauch Hit`
  (params (`Launch Hit` :type "/Game/ComboGame/Enum/E_LaunchHit Enum" :default "NewEnumerator2") (Actor :type "Actor Object Reference"))
  (returns (ReturnValue :type "Vector Structure"))
  (bind _asbp_third_person_character (cast `/Game/ComboGame/Character/BP_ThirdPersonCharacter` Actor))
  (bind _capsulecomponent (`Character.CapsuleComponent` _asbp_third_person_character))
  (bind _returnvalue (`SceneComponent.GetUpVector` _capsulecomponent))
  (bind _returnvalue_2 (`SceneComponent.GetRightVector` _capsulecomponent))
  (return (* (select `/Game/ComboGame/Enum/E_LaunchHit` (`local.Launch Hit`) :`NewEnumerator0` (`SceneComponent.GetForwardVector` _capsulecomponent) :`NewEnumerator3` _returnvalue :`NewEnumerator4` (* _returnvalue -1.0) :`NewEnumerator5` (* _returnvalue_2 -1.0) :`NewEnumerator6` _returnvalue_2) 750.0)))

(fn `Received_NotifyBegin`
  (params (MeshComp :type "SkeletalMeshComponent Object Reference") (Animation :type "AnimSequenceBase Object Reference") (TotalDuration :type "Float (single-precision)") (EventReference :type "AnimNotifyEventReference Structure (by ref)"))
  (returns (ReturnValue :type Boolean))
  (locals (L_Combo :type "/Game/ComboGame/Blueprint/AC_Combo Object Reference") (L_HitTrace :type "/Game/CT_Components/HitTraceSystem/Components/AC_HitTrace Object Reference"))
  (bind _returnvalue (`ActorComponent.GetOwner` MeshComp))
  (`KismetArrayLibrary.Array_Clear` (`self.As BP AI`))
  (set `local.L_Combo` (`Actor.GetComponentByClass` _returnvalue "/Game/ComboGame/Blueprint/AC_Combo.AC_Combo_C"))
  (set `local.L_HitTrace` (`Actor.GetComponentByClass` _returnvalue "/Game/CT_Components/HitTraceSystem/Components/AC_HitTrace.AC_HitTrace_C"))
  (`/Game/ComboGame/Blueprint/AC_Combo.SetBeginHitBox` (`local.L_Combo`) (`self.Hit Socket`))
  (`/Game/ComboGame/Blueprint/AC_Combo.SetComboWindow` (`local.L_Combo`) true)
  (`/Engine/EditorBlueprintResources/StandardMacros.IsValid` (`local.L_HitTrace`)
    (:`Is Valid`
      (add `/Game/CT_Components/HitTraceSystem/Components/AC_HitTrace.Event_OnHitActor` (`local.L_HitTrace`) (`|CreateDelegate` :!event `Event_OnHitActor`))
      (return false))))

(fn `Received_NotifyEnd`
  (params (MeshComp :type "SkeletalMeshComponent Object Reference") (Animation :type "AnimSequenceBase Object Reference") (EventReference :type "AnimNotifyEventReference Structure (by ref)"))
  (returns (ReturnValue :type Boolean))
  (bind _returnvalue (`ActorComponent.GetOwner` MeshComp))
  (bind ((`isWeapon_1_7B568DFF401F2BC1D259F2BB42B1A60D` _isweapon) (`isLeft_10_E00558D944E3B2B7DB9D1BA9D7952035` _isleft) (`LaunchHit_23_589ED3094B00984A041E2980C226C2B0` _launchhit)) (break `/Game/ComboGame/Struct/S_HitSocket` (`self.Hit Socket`)))
  (bind _returnvalue_2 (`Actor.GetComponentByClass` _returnvalue "/Game/ComboGame/Blueprint/AC_Combo.AC_Combo_C"))
  (`/Engine/EditorBlueprintResources/StandardMacros.IsValid` _returnvalue_2
    (:`Is Valid`
      (`/Game/ComboGame/Blueprint/AC_Combo.SetEndHitBox` _returnvalue_2 _isleft)
      (`/Game/ComboGame/Blueprint/AC_Combo.PlayNextCombo` _returnvalue_2 (`self.Combo End`) _isweapon)
      (`/Game/ComboGame/Blueprint/AC_Combo.SetComboWindow` _returnvalue_2 false)
      (bind _returnvalue_3 (`self.Lauch Hit` _launchhit _returnvalue))
      (`self.Hit ACtion` _returnvalue_3 _isweapon _returnvalue)
      (return false))
    (:`Is Not Valid`
      (return false))))