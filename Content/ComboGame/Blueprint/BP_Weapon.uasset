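; BP_Weapon is a weapon actor in ComboGame whose mesh and setup come from a data table.
; The construction script looks up the row named by its weapon name in DT_WeaponState and stores it as WeaponData.
; On BeginPlay it applies that row's static mesh to WeaponMesh and hides itself, with ShowWeapon toggling actor visibility.
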(event `self.ReceiveBeginPlay`
  (`StaticMeshComponent.SetStaticMesh` (`self.WeaponMesh`) (`.WeaponMesh_5_BE5367BD42A8479C5BE15A9889E653FD` (break `/Game/ComboGame/Struct/S_WeaponStruct` (`.WeaponSetup_21_FD76FC0642D3C7C7441FAEA543B8C51E` (break `/Game/ComboGame/Struct/S_WeaponState` (`self.Weapon Data`))))))
  (`self.Show Weapon` false))

(fn `Show Weapon`
  (params (`isShow?` :type Boolean))
  (`self.SetActorHiddenInGame` (not `isShow?`)))

(fn `UserConstructionScript`
  (bind _returnvalue (`|GetDataTableRow` "/Game/ComboGame/Datatable/DT_WeaponState.DT_WeaponState" (`.NameWeapon_2_E4A9EABB4873D78ECC633DA4AB1E251F` (break `/Game/ComboGame/Struct/S_WeaponStore` (`self.S Weapon Store`))))
    (:`then`
      (set `self.Weapon Data` _returnvalue))))