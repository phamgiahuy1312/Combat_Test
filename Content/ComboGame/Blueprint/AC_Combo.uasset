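; Character combat component that runs melee combos, dash and roll skills, and weapon spawning, equipping and swapping.
; Weapons from DT_WeaponState supply combo type, montages and ground or air combo data.
; Buffered inputs filter combo rows and queue montages played on notify; chained inputs step through light or heavy montages.
; It also drains stamina, shows inputs on a combo widget and drives AC_HitTrace hitboxes.
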(event `Init`
  (params (Mesh :type "SkeletalMeshComponent Object Reference"))
  ;[0.724 0.7396 0.203 0.5] Init
  (set `self.Mesh` Mesh)
  (`self.Reset Combo Data`)
  (for _array_element (`self.Weapons Store`)
    (bind _returnvalue (`|GetDataTableRow` "/Game/ComboGame/Datatable/DT_WeaponState.DT_WeaponState" (`.NameWeapon_2_E4A9EABB4873D78ECC633DA4AB1E251F` (break `/Game/ComboGame/Struct/S_WeaponStore` _array_element)))
      (:`then`
        (bind _returnvalue_2 (`|SpawnActorFromClass` "/Game/ComboGame/Blueprint/BP_Weapon.BP_Weapon_C" (`KismetMathLibrary.MakeTransform` (0.0 0.0 0.0)) "Undefined" "OverrideRootScale" (`self.GetOwner`) _array_element null))
        (`KismetArrayLibrary.Array_Add` (`self.Arr Weapons`) _returnvalue_2)
        (`Actor.K2_AttachToComponent` _returnvalue_2 (`self.Mesh`) (`.UnEquipSocket_10_74BCA82A4489AA81CB39C0AB5C807079` (break `/Game/ComboGame/Struct/S_WeaponStruct` (`.WeaponSetup_21_FD76FC0642D3C7C7441FAEA543B8C51E` (break `/Game/ComboGame/Struct/S_WeaponState` _returnvalue)))) "SnapToTarget" "SnapToTarget" "KeepRelative" true))))
  (set `self.Curent Weapon index` 0)
  (`KismetSystemLibrary.Delay` 0.2)
  (`self.Equip Weapon` 0)
  (`self.Change Weapon` 1)
  (set `self.Attribute` (`Actor.GetComponentByClass` (`self.GetOwner` (`self.Mesh`)) "/Game/ComboGame/Blueprint/Attribute/C_Attribute.C_Attribute_C")))

(event `Set Chained Attack`
  (bind _combo_max (`self.Get Chained Combo`))
  (bind _attack_index (`self.Attack Index`))
  (bind (_output_lightattack _output_heavyattack) (break `/Game/ComboGame/Struct/S_ChainedComboMontages` (`|GetArrayItem` (`.Combo Montages` (`self.Get Chained Combo`)) (`self.Attack Index`))))
  ;[0.4121 1 0.1668 0.7565] Set chained combo attack montages
  (if (== _attack_index _combo_max)
    (set `self.Attack Index` -1))
  (set `self.Attack Index` (`KismetMathLibrary.Clamp` (+ _attack_index 1) 0 _combo_max))
  (set `self.Light Chained Attack` _output_lightattack)
  (set `self.Heavy Chained Attack` _output_heavyattack))

(event `Equip Weapon`
  (params (`Weapon Index` :type Integer))
  (bind _equip_montage (`self.Equip Montage`))
  (bind _unequip_montage (`self.Unequip Montage`))
  ; Equip Weapon
  (set `self.Curent Weapon index` (`KismetMathLibrary.SelectInt` `Weapon Index` 0 (`self.is Weapon`)))
  (if (`KismetSystemLibrary.IsValid` (`self.Current Weapon`))
    (`/Engine/EditorBlueprintResources/StandardMacros.IsValid` _unequip_montage
      (:`Is Valid`
        (`self.Play Montage` _unequip_montage 1.0)
        (`KismetSystemLibrary.Delay` (* (`AnimSequenceBase.SequenceLength` (`self.Unequip Montage`)) 0.8)))
      (:`Is Not Valid`
        _)))
  (bind _output_get (set `self.Current Weapon` (`|GetArrayItem` (`self.Arr Weapons`) (`self.Curent Weapon index`))))
  (`/Engine/EditorBlueprintResources/StandardMacros.IsValid` _output_get
    (:`Is Valid`
      (`self.Set Weapon Variables`)
      (`self.Reset Combo Data`)
      (`/Engine/EditorBlueprintResources/StandardMacros.IsValid` _equip_montage
        (:`Is Valid`
          (`self.Play Montage` _equip_montage 1.0))
        (:`Is Not Valid`
          (`self.Set Weapon State`))))))

(event `Cycle Weapons`
  ; Cycle Weapons
  (set `self.is Weapon` (not (`self.is Weapon`)))
  (`self.Equip Weapon` (`self.Weapon Index`)))

(event `Play Chained Attack`
  (params (Montage :type "AnimMontage Object Reference"))
  ;[0.4121 1 0.1668 0.7565] Play chained combo attack montages
  (`|PlayMontage` (`self.Mesh`) Montage 1.5
    (:`then`
      (if (`self.Is in Air?`)
        (`self.SetMovementMode` "MOVE_Flying")))
    (:`OnCompleted`
      (set `self.Attack Index` -1)
      (`/Game/ComboGame/UI/WG_Combo_Main.ClearComboInput` (`self.WG Combo`))
      (set `self.Input Index` -1)
      (set `self.Combo Data Index` 0))
    (:`OnInterrupted`
      (if (== (`self.Attack Index`) (`self.Get Chained Combo`))
        (set `self.Attack Index` -1 :!label _label)
        (`/Game/ComboGame/UI/WG_Combo_Main.ClearComboInput` (`self.WG Combo`))
        (if (`self.Is in Air?`)
          (`self.SetMovementMode` "MOVE_Falling"))))
    (:`OnNotifyBegin`
      (goto _label))))

(event `Set WG Combo`
  (params (`WG Combo` :type "/Game/ComboGame/UI/WG_Combo_Main Object Reference"))
  (set `self.WG Combo` `WG Combo`))

(event `Play Skill Montage`
  (params (`is Dash` :type Boolean))
  (bind (_anim_roll _anim_dash) (`self.Get Anim`))
  ; Skill
  (`/Engine/EditorBlueprintResources/StandardMacros.DoOnce` false :!label _label_2
    (:`Completed`
      (`/Game/ComboGame/Blueprint/Attribute/C_Attribute.IncVariable` (`self.Attribute`) (struct :`TagName` "Attribute.Dynamic.Stamina") -15.0)
      (`|PlayMontage` (`self.Mesh`) (select `bool` `is Dash` :`false` _anim_roll :`true` _anim_dash) 1.5
        (:`then`
          (`KismetSystemLibrary.RetriggerableDelay` 0.8)
          (goto _label_2 :!via `Reset`))))))

(event `Play Montage`
  (params (MontageToPlay :type "AnimMontage Object Reference") (InPlayRate :type "Float (single-precision)"))
  ; Play Anim Montage
  (`|PlayMontage` (`self.Mesh`) MontageToPlay 1.5
    (:`then`
      (if (`self.Is in Air?`)
        (`self.SetMovementMode` "MOVE_Flying")
        (if (`self.Is in Air?`)
          (`self.SetMovementMode` "MOVE_Falling"))))
    (:`OnCompleted`
      (`self.Reset Combo Data` :!label _label_3))
    (:`OnNotifyBegin`
      (goto _label_3))))

(event `PlayCombo`
  ; If combo input is matched we cycle anim montage. PlayNextCombo is called using a notify (Combo_Notify)
  (`self.Play Montage` (`|GetArrayItem` (`self.Combo Montages`)) 1.0 :!label _label_4)
  (`KismetArrayLibrary.Array_Remove` (`self.Combo Montages`))
  (set `self.Movement Mode` (`self.GetCurrentMovementMode`)))

(event `PlayNextCombo`
  (params (`Combo End` :type Boolean) (isWeapon :type Boolean))
  ; If combo input is matched we cycle anim montage. PlayNextCombo is called using a notify (Combo_Notify)
  (if (not isWeapon)
    (if (not `Combo End`)
      (if (> (`KismetArrayLibrary.Array_Length` (`self.Combo Montages`)) 0)
        (goto _label_4)
        (else
          _)))
    (`self.Reset Combo Data`)))

(event `Lauch Hit`
  (params (LaunchVelocity :type "Vector Structure"))
  (bind _ascharacter (cast `Character` (`self.GetOwner`)))
  (`Character.LaunchCharacter` _ascharacter LaunchVelocity true true))

(event `Reset Movement`
  (params (Duration :type "Float (double-precision)") (Character :type "CharacterMovementComponent Object Reference"))
  (`KismetSystemLibrary.RetriggerableDelay` (+ Duration 0.2))
  (`CharacterMovementComponent.SetMovementMode` Character "MOVE_Falling" 0)
  (set `CharacterMovementComponent.GravityScale` 1.0 Character))

(fn `Action Equip Weapon`
  (bind _current_weapon (`self.Current Weapon`))
  (`/Engine/EditorBlueprintResources/StandardMacros.IsValid` _current_weapon
    (:`Is Valid`
      (`Actor.K2_AttachToComponent` _current_weapon (`self.Mesh`) (`self.Equip Socket`) "KeepRelative" "KeepRelative" "KeepRelative" true)
      (message `/Game/ComboGame/Blueprint/Interface/BPI_CharacterAnimation.Toggle Melee Weapon` (`SkeletalMeshComponent.GetAnimInstance` (`self.Mesh`)) true))))

(fn `Action UnEquip Weapon`
  (bind _current_weapon (`self.Current Weapon`))
  (`/Engine/EditorBlueprintResources/StandardMacros.IsValid` _current_weapon
    (:`Is Valid`
      (`Actor.K2_AttachToComponent` _current_weapon (`self.Mesh`) (`self.Un Equip Socket`) "KeepRelative" "KeepRelative" "KeepRelative" true)
      (message `/Game/ComboGame/Blueprint/Interface/BPI_CharacterAnimation.Toggle Melee Weapon` (`SkeletalMeshComponent.GetAnimInstance` (`self.Mesh`)) false))))

(fn `ActionChangeWeapon`
  (if (not (`self.is Weapon`))
    (`self.Change Weapon` (select `bool` (== (`self.Weapon Index`) 1) :`false` 1 :`true` 2))))

(fn `Change Weapon`
  (params (`Weapon Index` :type Integer))
  (locals (`L Current Weapon` :type Integer))
  (bind _output (`|GetArrayItem` (`self.Arr Weapons`) (`self.Weapon Index`)))
  (bind _output_2 (`|GetArrayItem` (`self.Arr Weapons`) (`local.L Current Weapon`)))
  (set `local.L Current Weapon` (`self.Weapon Index`))
  (set `self.Weapon Index` `Weapon Index`)
  (`|ExecutionSequence`
    (:`then_0`
      (`/Engine/EditorBlueprintResources/StandardMacros.IsValid` _output_2
        (:`Is Valid`
          (`/Game/ComboGame/Blueprint/BP_Weapon.Show Weapon` _output_2 false))))
    (:`then_1`
      (`/Engine/EditorBlueprintResources/StandardMacros.IsValid` _output
        (:`Is Valid`
          (`/Game/ComboGame/Blueprint/BP_Weapon.Show Weapon` _output true))))))

(fn `ComboInput`
  (params (`Combo Type` :type "/Game/ComboGame/Enum/E_ComboInput Enum" :default "NewEnumerator2") (IsPressed :type Boolean))
  (bind _returnvalue (select `/Game/ComboGame/Enum/E_ComboInput` (`self.Combo Input`) :`NewEnumerator0` (`self.Light Chained Attack`) :`NewEnumerator1` (`self.Heavy Chained Attack`)))
  (set `self.Combo Input` `Combo Type`)
  (bind _output_get (set `self.IsPressed` IsPressed))
  (if _output_get
    (switch `/Game/ComboGame/Enum/E_ComboType` (`self.Combo Type`)
      (:`NewEnumerator2`
        (switch `/Game/ComboGame/Enum/E_ActionState` (`self.Action State`)
          (:`NewEnumerator0`
            (set `self.Is Combo Open` true))
          (:`NewEnumerator1`
            _))
        (if (`self.Is Combo Open`)
          (if (not (`|EnumEquality` (`self.GetCurrentMovementMode`) (`self.Movement Mode`)))
            (`self.Reset Combo Data`))
          (`/Engine/EditorBlueprintResources/StandardMacros.IncrementInt` (`self.Input Index`)
            (:`  `
              (`self.Loop Combos`
                (:`true`
                  (`self.ProceedWithComboAnim`)
                  (`/Game/ComboGame/Blueprint/Attribute/C_Attribute.IncVariable` (`self.Attribute`) (struct :`TagName` "Attribute.Dynamic.Stamina") -5.0 :!label _label))
                (:`false`
                  (`self.CheckNextCombo`
                    (:`Found Is Combo`
                      (`self.ProceedWithComboAnim`)
                      (goto _label))
                    (:`Not Found Combo`
                      (`self.Reset Combo Data`)))))))))
      (:`NewEnumerator0`
        (`/Engine/EditorBlueprintResources/StandardMacros.IncrementInt` (`self.Input Index`)
          (:`  `
            (`self.Loop Combos`
              (:`true`
                (`/Game/ComboGame/UI/WG_Combo_Main.AddComboInput` (`self.WG Combo`) (`self.Combo Input`) (`self.Get Combo Data`) :!label _label_2))
              (:`false`
                (`self.CheckNextCombo`
                  (:`Found Is Combo`
                    (goto _label_2))
                  (:`Not Found Combo`
                    (`self.Reset Combo Data`)))))
            (`self.Set Chained Attack`)
            (`/Engine/EditorBlueprintResources/StandardMacros.IsValid` _returnvalue
              (:`Is Valid`
                (`self.Play Chained Attack` _returnvalue)
                (`/Game/ComboGame/Blueprint/Attribute/C_Attribute.IncVariable` (`self.Attribute`) (struct :`TagName` "Attribute.Dynamic.Stamina") -10.0)))))))))

(fn `Get Action State`
  (returns (`Action State` :type "/Game/ComboGame/Enum/E_ActionState Enum"))
  (return (`self.Action State`)))

(fn `Get Anim`
  (returns (`Anim Roll` :type "AnimMontage Object Reference") (`Anim Dash` :type "AnimMontage Object Reference"))
  (if (`self.is Weapon`)
    (if (`self.Is in Air?`)
      (return "/Game/ComboGame/Character/Animations/Sequence/05_Jump/02_Jump_Combat/02_Jump_Combat_F_0/Jump_Combat_Start_F_0_Seq_Montage.Jump_Combat_Start_F_0_Seq_Montage" "/Game/ComboGame/Character/Animations/Sequence/06_Dodge/04_Dodge_Air_Combat/Dodge_Air_Combat_F_Seq_Montage.Dodge_Air_Combat_F_Seq_Montage")
      (else
        (return "/Game/ComboGame/Character/Animations/Sequence/07_Roll/02_Roll_Combat/Roll_Combat_F_0_Seq_Montage.Roll_Combat_F_0_Seq_Montage" "/Game/ComboGame/Character/Animations/Sequence/06_Dodge/05_Dodge_to_Run/Dodge_to_Run_F_Seq_Montage.Dodge_to_Run_F_Seq_Montage")))
    (elif (`self.Is in Air?`)
      (return "/Game/ComboGame/Character/Animations/Sequence/05_Jump/02_Jump_Combat/02_Jump_Combat_F_0/Jump_Combat_Start_F_0_Seq_Montage.Jump_Combat_Start_F_0_Seq_Montage" "/Game/ComboGame/Character/Animations/Sequence/06_Dodge/03_Dodge_Air/Dodge_Air_F_Seq_Montage.Dodge_Air_F_Seq_Montage")
      (else
        (return "/Game/ComboGame/Character/Animations/Sequence/07_Roll/01_Roll/Roll_F_0_Seq_Montage.Roll_F_0_Seq_Montage" "/Game/ComboGame/Character/Animations/Sequence/06_Dodge/01_Dodge/Doge_F_Seq_Montage.Doge_F_Seq_Montage")))))

(fn `Get Combo Data`
  (returns (Name :type Name) (`Combo Input` :type "Array of /Game/ComboGame/Enum/E_ComboInput Enum") (`Combo Montage` :type "Array of AnimMontage Object Reference"))
  (bind (_name _comboinput _combomontage) (break `/Game/ComboGame/Struct/S_BufferedCombo` (`|GetArrayItem` (`self.ComboStruct`) (`self.Combo Data Index`))))
  (return _name _comboinput _combomontage))

(fn `Get Name Combo`)

(fn `GetCurrentMovementMode`
  (returns (MovementMode :type "EMovementMode Enum"))
  (return (`CharacterMovementComponent.MovementMode` (`Actor.GetComponentByClass` (`self.GetOwner`) "/Script/Engine.CharacterMovementComponent"))))

(fn `Play Sound Not Hit`
  (params (`is Weapon` :type Boolean))
  (`GameplayStatics.PlaySound2D` (select `bool` `is Weapon` :`false` "/Game/CombatTest/Audio/Action/Punch.Punch" :`true` "/Game/CombatTest/Audio/Action/whoosh-sfx.whoosh-sfx" :!type "SoundBase Object Reference") 0.5 0.5 0.2 null null))

(fn `ProceedWithComboAnim`
  (bind (_name _combo_input _combo_montage) (`self.Get Combo Data`))
  (`KismetArrayLibrary.Array_Add` (`self.Combo Montages`) (`|GetArrayItem` _combo_montage (`self.Input Index`)))
  (switch `/Game/ComboGame/Enum/E_ActionState` (`self.Action State`)
    (:`NewEnumerator0`
      (`self.PlayCombo`))
    (:`NewEnumerator1`
      _))
  (`/Game/ComboGame/UI/WG_Combo_Main.AddComboInput` (`self.WG Combo`) (`self.Combo Input`) _name))

(fn `Reset Combo Data`
  (bind _wg_combo (`self.WG Combo`))
  (`/Engine/EditorBlueprintResources/StandardMacros.IsValid` _wg_combo
    (:`Is Valid`
      (`/Game/ComboGame/UI/WG_Combo_Main.ClearComboInput` _wg_combo))
    (:`Is Not Valid`
      _))
  (`|ExecutionSequence`
    (:`then_0`
      (`KismetArrayLibrary.Array_Clear` (`self.ComboStruct`))
      (`KismetArrayLibrary.Array_Clear` (`self.Combo Montages`)))
    (:`then_1`
      (bind _output_get (set `self.CurrentData` (select `bool` (`self.Is in Air?`) :`false` (`self.Ground Combo Data`) :`true` (`self.Air Combo Data`))))
      (bind _outrownames (`DataTableFunctionLibrary.GetDataTableRowNames` _output_get))
      (for _array_element _outrownames
        (bind _returnvalue (`|GetDataTableRow` (`self.CurrentData`) _array_element)
          (:`then`
            (bind _structout (setmembers `/Game/ComboGame/Struct/S_BufferedCombo` :`StructRef` _returnvalue))
            (`KismetArrayLibrary.Array_Add` (`self.ComboStruct`) _structout)))))
    (:`then_2`
      (set `self.Input Index` -1)
      (set `self.Combo Data Index` 0))))

(fn `Set Action State`
  (params (`Action State` :type "/Game/ComboGame/Enum/E_ActionState Enum" :default "NewEnumerator0"))
  (set `self.Action State` `Action State`))

(fn `Set Weapon State`
  (set `self.Weapon State` (`.WeaponState_2_5EC826A4401388F2E1985B862A1C3946` (break `/Game/ComboGame/Struct/S_WeaponStruct` (`.WeaponSetup_21_FD76FC0642D3C7C7441FAEA543B8C51E` (break `/Game/ComboGame/Struct/S_WeaponState` (`/Game/ComboGame/Blueprint/BP_Weapon.Weapon Data` (`self.Current Weapon`))))))))

(fn `Set Weapon Variables`
  (bind (_weaponsetup _combosetup _actionsmontages _skillweapon) (break `/Game/ComboGame/Struct/S_WeaponState` (`/Game/ComboGame/Blueprint/BP_Weapon.Weapon Data` (`self.Current Weapon`))))
  (bind ((`EquipSocket_8_CBAAFDAF424BA3FDD38577A0961345DC` _equipsocket) (`UnEquipSocket_10_74BCA82A4489AA81CB39C0AB5C807079` _unequipsocket)) (break `/Game/ComboGame/Struct/S_WeaponStruct` _weaponsetup))
  (bind (_combotype _bufferedcomboattacks _chainedcomboattacks) (break `/Game/ComboGame/Struct/S_ComboStruct` _combosetup))
  (bind (_equipmontage _unequipmontage) (break `/Game/ComboGame/Struct/S_ActionStruct` _actionsmontages))
  (bind (_groundcomboattacks _aircomboattacks) (break `/Game/ComboGame/Struct/S_ChainedComboAttacks` _chainedcomboattacks))
  (bind (_groundcombodata _aircombodata _crouchingcombodata) (break `/Game/ComboGame/Struct/S_BuffredComboAttacks` _bufferedcomboattacks))
  (set `self.Equip Socket` _equipsocket)
  (set `self.Un Equip Socket` _unequipsocket)
  (set `self.Combo Type` _combotype)
  (set `self.Ground Combo Data` _groundcombodata)
  (set `self.Air Combo Data` _aircombodata)
  (set `self.Crouching Combo Data` _crouchingcombodata)
  (set `self.Ground Combo Attack` _groundcomboattacks)
  (set `self.Air Combo Attacks` _aircomboattacks)
  (set `self.Equip Montage` _equipmontage)
  (set `self.Unequip Montage` _unequipmontage)
  (set `self.Skill Weapon` _skillweapon))

(fn `SetBeginHitBox`
  (params (`Hit Socket` :type "/Game/ComboGame/Struct/S_HitSocket Structure"))
  (locals (`Hit Trace` :type "/Game/CT_Components/HitTraceSystem/Components/AC_HitTrace Object Reference") (Actor :type "Actor Object Reference"))
  (bind (_isweapon _isleft _begin_l_socket _end_l_socket _isright _begin_r_socket _end_r_socket) (break `/Game/ComboGame/Struct/S_HitSocket` (`local.Hit Socket`)))
  (bind _returnvalue (`self.GetOwner` (`self.Mesh`)))
  (set `local.Actor` _returnvalue)
  (set `local.Hit Trace` (`Actor.GetComponentByClass` _returnvalue "/Game/CT_Components/HitTraceSystem/Components/AC_HitTrace.AC_HitTrace_C"))
  (`|ExecutionSequence`
    (:`then_0`
      (if _isleft
        (`/Game/CT_Components/HitTraceSystem/Components/AC_HitTrace.BeginTraceByChannel` (`local.Hit Trace`) "Left" (select `bool` _isweapon :`false` (`self.Mesh`) :!type "SceneComponent Object Reference") (`KismetStringLibrary.Conv_StringToName` (`|GetEnumeratorNameAsString` _begin_l_socket)) (`KismetStringLibrary.Conv_StringToName` (`|GetEnumeratorNameAsString` _end_l_socket)) (`|MakeArray` (`local.Actor`)) 1.0 "TraceTypeQuery1" false "None" true (`local.Actor`))))
    (:`then_1`
      (if _isright
        (`/Game/CT_Components/HitTraceSystem/Components/AC_HitTrace.BeginTraceByChannel` (`local.Hit Trace`) "Right" (select `bool` _isweapon :`false` (`self.Mesh`) :`true` (`/Game/ComboGame/Blueprint/BP_Weapon.WeaponMesh` (`self.Current Weapon`)) :!type "SceneComponent Object Reference") (`KismetStringLibrary.Conv_StringToName` (`|GetEnumeratorNameAsString` _begin_r_socket)) (`KismetStringLibrary.Conv_StringToName` (`|GetEnumeratorNameAsString` _end_r_socket)) (`|MakeArray` (`local.Actor`)) 1.0 "TraceTypeQuery1" false "None" true (`local.Actor`))))))

(fn `SetComboWindow`
  (params (`Is Combo Open` :type Boolean))
  (set `self.Is Combo Open` `Is Combo Open`))

(fn `SetEndHitBox`
  (params (isLeft :type Boolean))
  (locals (`Hit Trace` :type "/Game/CT_Components/HitTraceSystem/Components/AC_HitTrace Object Reference"))
  (set `local.Hit Trace` (`Actor.GetComponentByClass` (`self.GetOwner` (`self.Mesh`)) "/Game/CT_Components/HitTraceSystem/Components/AC_HitTrace.AC_HitTrace_C"))
  (`/Game/CT_Components/HitTraceSystem/Components/AC_HitTrace.EndTrace` (`local.Hit Trace`) (select `bool` (`local.isLeft`) :`false` "Right" :`true` "Left" :!type "Name")))

(fn `SetMovementMode`
  (params (NewMovementMode :type "EMovementMode Enum" :default "MOVE_None"))
  (`CharacterMovementComponent.SetMovementMode` (`Actor.GetComponentByClass` (`self.GetOwner`) "/Script/Engine.CharacterMovementComponent") NewMovementMode 0))