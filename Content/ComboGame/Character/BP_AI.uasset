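; AI character Blueprint for the combo game that handles reactions to being hit.
; HitAction plays a hit montage, passes damage as a multiplier to RegenHelth for the health attribute, then uses the ACCombo component to launch the character and reset movement.
; A separate event activates blood VFX, and PlaySoundHit picks a weapon or punch sound.
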(event `self.ReceiveBeginPlay`
  (`parent.ReceiveBeginPlay`))

(event `Hit VFX Blood`
  (`ActorComponent.Activate` (`self.Blood`) true))

(fn `Hit Action`
  (params (Dame :type "Float (double-precision)") (`Lauch Velocity` :type "Vector Structure") (Weapon :type Boolean))
  (set `self.Dame` Dame)
  (`AnimInstance.Montage_Play` (`SkeletalMeshComponent.GetAnimInstance` (`self.Mesh`)) "/Game/ComboGame/Character/Animations/Hit_L_Seq_Montage.Hit_L_Seq_Montage" 1.0 "MontageLength" 0.0 true)
  (`|ExecutionSequence`
    (:`then_0`
      (`self.RegenHelth` (`self.Dame`))
      (`/Game/ComboGame/Blueprint/AC_Combo.Lauch Hit` (`self.AC_Combo`) (`local.Lauch Velocity`)))
    (:`then_1`
      (`/Game/ComboGame/Blueprint/AC_Combo.Reset Movement` (`self.AC_Combo`) 0.0 (`self.CharacterMovement`)))))

(fn `Play Sound Hit`
  (params (`is Weapon` :type Boolean))
  (`GameplayStatics.PlaySound2D` (select `bool` `is Weapon` :`false` "/Game/CombatTest/Audio/Action/Punch.Punch" :`true` "/Game/CombatTest/Audio/Action/HIT.HIT" :!type "SoundBase Object Reference") 1.25 1.0 0.2 null null))

(fn `RegenHelth`
  (params (MultiplyValue :type "Float (double-precision)"))
  (`parent.RegenHelth` MultiplyValue))

(fn `RegenHelth_`
  (params (MultiplyValue :type "Float (double-precision)"))
  (`/Game/ComboGame/Blueprint/Attribute/C_Attribute.IncVariable` (`self.C_Attribute`) (struct :`TagName` "Attribute.Dynamic.Health") (* (`/Game/ComboGame/Blueprint/Attribute/C_Attribute.GetAttribute` (`self.C_Attribute`) (struct :`TagName` "Attribute.Regen.Health")) (`local.MultiplyValue`))))

(fn `UserConstructionScript`
  (`parent.UserConstructionScript`))